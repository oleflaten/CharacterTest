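; Enemy character Blueprint that senses the player through AI Perception and feeds the results to its Behavior Tree via the Blackboard.
; Each perception update on the main character stores their location as PlayerLocation, then sets PlayerHeard for "Noise"-tagged stimuli or PlayerSpotted for others, using the sensed state.
; Tick manually turns the mesh to face movement velocity with a -90 yaw offset, working around rotation broken under Behavior Trees.
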(event `self.ReceiveTick`
  (params (DeltaSeconds :type "Float (single-precision)"))
  (bind _velocity (`MovementComponent.Velocity` (`self.CharacterMovement`)))
  ;[1 1 1] For some reason the rotation of the character broke when using Behavior trees
  (if (> (`KismetMathLibrary.VSize` _velocity) 0.1)
    (`SceneComponent.K2_SetWorldRotation` (`self.Mesh`) (`KismetMathLibrary.ComposeRotators` (`KismetMathLibrary.Conv_VectorToRotator` _velocity) (struct :`Yaw` -90.0)) false false)))

(event `self.AIPerception.OnTargetPerceptionUpdated`
  (params (Actor :type "Actor Object Reference") (Stimulus :type "AIStimulus Structure"))
  (bind (_age _expirationage _strength _stimuluslocation _receiverlocation _tag _bsuccessfullysensed) (break `AIStimulus` Stimulus))
  ;[1 1 1] Sense something
  (bind _asmain_character_bp (cast `/Game/Blueprints/MainCharacter_BP` Actor))
  (`BlackboardComponent.SetValueAsVector` (`AIBlueprintHelperLibrary.GetBlackboard` null) "PlayerLocation" (`self.K2_GetActorLocation` _asmain_character_bp))
  (if (== _tag "Noise")
    ;[1 1 1] Hear noise
    (`BlackboardComponent.SetValueAsBool` (`AIBlueprintHelperLibrary.GetBlackboard` null) "PlayerHeard" _bsuccessfullysensed)
    (`KismetSystemLibrary.PrintString` "Player Heard")
    (else
      ;[1 1 1] Player Spotted
      (`BlackboardComponent.SetValueAsBool` (`AIBlueprintHelperLibrary.GetBlackboard` null) "PlayerSpotted" _bsuccessfullysensed)
      (`KismetSystemLibrary.PrintString` "PlayerSeen"))))

(fn `UserConstructionScript`)